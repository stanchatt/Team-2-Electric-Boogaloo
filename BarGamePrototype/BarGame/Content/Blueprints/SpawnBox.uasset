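; SpawnBox is an actor that spawns a single object of a configurable class at a random point within its box volume.
; On BeginPlay it waits a random delay between MinDelay and MaxDelay, then calls SpawnItem once.
; SpawnItem picks random X and Y offsets within the scaled box extent and adds them to the actor location, ignoring box height and actor rotation.
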(event `self.ReceiveBeginPlay`
  (`KismetSystemLibrary.Delay` (`KismetMathLibrary.RandomFloatInRange` (`self.MinDelay`) (`self.MaxDelay`)))
  (`self.SpawnItem`))

(fn `SpawnItem`
  (bind _x (.x (`BoxComponent.GetScaledBoxExtent` (`self.Volume`))))
  (bind _y (.y (`BoxComponent.GetScaledBoxExtent` (`self.Volume`))))
  (`|SpawnActorFromClass` (`self.Object Spawn`) (`KismetMathLibrary.MakeTransform` (+ (`KismetMathLibrary.MakeVector` (`KismetMathLibrary.RandomFloatInRange` (* _x -1.0) _x) (`KismetMathLibrary.RandomFloatInRange` (* _y -1.0) _y)) (`self.K2_GetActorLocation`))) "Undefined" "OverrideRootScale" null null))

(fn `UserConstructionScript`)